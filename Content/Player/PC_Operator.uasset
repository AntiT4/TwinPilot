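; Player controller for the operator in a Pixel Streaming app, handling cursor selection plus rotate and pan input.
; BeginPlay adds the Enhanced Input context and caps frame rate; rotate and pan actions set held flags.
; Select either confirms the actor under the cursor and moves P_Operator toward it, or just selects.
; Both paths send the client JSON naming selected, confirmed and released actors; custom cursor code is disconnected.
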(event Input|EnhancedActionEvents|EnhancedInputActionIA_Pan
  (params (ActionValue :type Boolean) (ElapsedSeconds :type Float%20%28double-precision%29) (TriggeredSeconds :type Float%20%28double-precision%29) (InputAction :type Input%20Action%20Object%20Reference :default "/TwinPilot/Player/Inputs/IA_Pan.IA_Pan"))
  (:Started
    (Class|DigitalTwinOperatorController|SetPanHeld true))
  (:Completed
    (Class|DigitalTwinOperatorController|SetPanHeld false)))

(event Input|EnhancedActionEvents|EnhancedInputActionIA_ApplyRotation
  (params (ActionValue :type Boolean) (ElapsedSeconds :type Float%20%28double-precision%29) (TriggeredSeconds :type Float%20%28double-precision%29) (InputAction :type Input%20Action%20Object%20Reference :default "/TwinPilot/Player/Inputs/IA_ApplyRotation.IA_ApplyRotation"))
  (Class|DigitalTwinOperatorController|SetRotateHeld ActionValue))

(event Input|EnhancedActionEvents|EnhancedInputActionIA_Select
  (params (ActionValue :type Boolean) (ElapsedSeconds :type Float%20%28double-precision%29) (TriggeredSeconds :type Float%20%28double-precision%29) (InputAction :type Input%20Action%20Object%20Reference :default "/TwinPilot/Player/Inputs/IA_Select.IA_Select"))
  (bind _lastinteractionstatechange (Variables|Default|GetLastInteractionStateChange))
  (bind (_previousstate _currentstate) (Utilities|Struct|BreakTwinPilotInteractionStateChange _lastinteractionstatechange))
  (bind (_selectedactor _selectedhighlightedactor _confirmedactor _confirmedhighlightedactor) (Utilities|Struct|BreakTwinPilotInteractionState _currentstate))
  (Utilities|FlowControl|Sequence
    (:then_0
      (bind _returnvalue (Class|DigitalTwinOperatorController|ConfirmActorUnderCursor))
      (if _returnvalue
        (bind _asp_operator (Utilities|Casting|CastToP_Operator (Game|Player|GetPlayerPawn 0)))
        (Class|DigitalTwinOperatorPawn|GoTowardActor _asp_operator (Class|DigitalTwinOperatorController|GetConfirmedActor))
        (else
          (Class|DigitalTwinOperatorController|SelectUnderCursor)))
      ;[0.15 0.15 0.15 0.5] Send Client Confirmed Actor/Released Actor Data
      (Class|PixelStreaming2Input|SendPixelStreaming2Response (Variables|Default|GetPixelStreaming2Input) (.OutJsonString (Class|DigitalTwinJsonBlueprintLibrary|JsonObjecttoStringPure (.OutJsonObject (Class|DigitalTwinJsonBlueprintLibrary|SetJsonFieldPure (.OutJsonObject (Class|DigitalTwinJsonBlueprintLibrary|SetJsonFieldPure (.OutJsonObject (Class|DigitalTwinJsonBlueprintLibrary|SetJsonFieldPure (.OutJsonObject (Class|DigitalTwinJsonBlueprintLibrary|SetJsonStringFieldPure (Class|DigitalTwinJsonBlueprintLibrary|MakeEmptyJsonObject) "event" "mouse_click")) "selected_actor" (CallFunction|MakeJsonObject _selectedactor))) "confirmed_actor" (CallFunction|MakeJsonObject _confirmedhighlightedactor))) "relesed_actor" (CallFunction|MakeJsonObject (.ConfirmedHighlightedActor (Utilities|Struct|BreakTwinPilotInteractionState _previousstate)))))))))))

(event EventBeginPlay
  (Input|AddMappingContext (PlayerController|LocalPlayerSubsystems|GetEnhancedInputLocalPlayerSubsystem) "/TwinPilot/Player/Inputs/MC_Operator.MC_Operator" 0 "(bIgnoreAllPressedKeysUntilRelease=True,bForceImmediately=False,bNotifyUserSettings=False)")
  (Development|ExecuteConsoleCommand "t.MaxFPS 60" self))

(event Input|KeyboardEvents|DebugKeyQ
  (params (Key :type Key%20Structure :default "None") (ActionValue :type Input%20Action%20Value%20Structure)))

(fn ConstructionScript)

(fn MakeJsonObject
  (params (Object :type Object%20Object%20Reference))
  (return (.OutJsonObject (Class|DigitalTwinJsonBlueprintLibrary|SetJsonStringFieldPure (Class|DigitalTwinJsonBlueprintLibrary|MakeEmptyJsonObject) "name" (Utilities|GetDisplayName Object)))))